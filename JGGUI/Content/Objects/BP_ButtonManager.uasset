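; BP_ButtonManager manages a group of buttons as a single selection, with each button mapped to an enum value.
; Setup binds a press handler to every key in the Buttons map and disables the initially selected button.
; A press re-enables the previous selection, optionally disables the pressed button, and stores it as selected.
; It then calls ButtonPressed with the new and old enum values.
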(event Custom|Setup
  (bind _buttons (Variables|Default|GetButtons))
  (bind _selectedbutton (Variables|Default|GetSelectedButton))
  (bind (_value _returnvalue) (Utilities|Map|Find _buttons _selectedbutton))
  (Utilities|FlowControl|Sequence
    (:then_0
      (bind _keys (Utilities|Map|Keys (Variables|Default|GetButtons)))
      (for _array_element _keys
        (EventDispatchers|AssignButtonPressed _array_element (delegate Custom|OnTargetButtonPressed))))
    (:then_1
      (if _returnvalue
        (Variables|Default|SetSelectedButtonEnum _value)
        (Default|SetButtonEnabled (Variables|Default|GetSelectedButton) false)))))

(event Custom|OnTargetButtonPressed
  (params (Button :type WB%20Button%20Object%20Reference))
  (bind _buttons (Variables|Default|GetButtons))
  (bind (_value _returnvalue) (Utilities|Map|Find _buttons Button))
  (if _returnvalue
    (Utilities|FlowControl|Sequence
      (:then_0
        (if (Variables|Default|GetbDisableAfterPress)
          (Default|SetButtonEnabled Button false)))
      (:then_1
        (Utilities|IsValid (Variables|Default|GetSelectedButton)
          (:Is%20Valid
            (Default|SetButtonEnabled (Variables|Default|GetSelectedButton) true))))
      (:then_2
        (Variables|Default|SetSelectedButton Button)
        (bind _output_get (Variables|Default|SetPreviousButtonEnum (Variables|Default|GetSelectedButtonEnum)))
        (bind _output_get_2 (Variables|Default|SetSelectedButtonEnum _value))
        (Default|CallButtonPressed _output_get_2 _output_get)))))