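; Base tutorial component that steps through a sequence, showing step text and playing dialogue through a supplied dialogue component.
; Next and previous functions move the step index; first runs update non-empty title and description, while reruns prefer rerun dialogue, falling back to the first.
; UpdateStepEnum, OnAllDialogueFinished and IsObjectiveValid are stubs, apparently for child overrides; EndStep advances to the next step.
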(event EventBeginPlay)

(event EventTick
  (params (DeltaSeconds :type Float%20%28single-precision%29)))

(fn Setup
  (params (DialogueComponent :type BP%20Dialogue%20Component%20Object%20Reference) (TitleTextBlock :type Text%20Block%20Object%20Reference) (DescTextBlock :type Text%20Block%20Object%20Reference))
  (Utilities|FlowControl|Sequence
    (:then_0
      (bind _output_get (Variables|Variable|SetDialogueComponent DialogueComponent))
      (EventDispatchers|BindEventtoAllDialogueFinished _output_get (EventDispatchers|CreateEvent :!event OnAllDialogueFinished)))
    (:then_1
      (bind _output_get_2 (Variables|Variable|SetTitleTextBlock TitleTextBlock))
      (Utilities|IsValid _output_get_2
        (:Is%20Valid
          (Variables|/Script/UMG.TextBlock|SetText _output_get_2 ""))))
    (:then_2
      (bind _output_get_3 (Variables|Variable|SetDescTextBlock DescTextBlock))
      (Utilities|IsValid _output_get_3
        (:Is%20Valid
          (Variables|/Script/UMG.TextBlock|SetText _output_get_3 ""))))))

(fn StartTutorial
  (Variables|Variable|SetCurrentStepIndex -1)
  (CallFunction|CheckforNextStep))

(fn GetCurrentStepIndex
  (return (Variables|Variable|GetCurrentStepIndex)))

(fn CheckforPreviousStep
  (CallFunction|SetupPreviousStep)
  (if (>= (Variables|Variable|GetCurrentStepIndex) 0)
    (CallFunction|RerunStep)))

(fn CheckforNextStep
  (CallFunction|SetupNextStep)
  (if (CallFunction|IsObjectiveValid)
    (CallFunction|RunStepFirstTime)))

(fn SetupPreviousStep
  (Math|Integer|DecrementInt (Variables|Variable|GetCurrentStepIndex)
    (:%20%20
      (CallFunction|UpdateStepEnum))))

(fn SetupNextStep
  (Math|Integer|IncrementInt (Variables|Variable|GetCurrentStepIndex)
    (:%20%20
      (CallFunction|UpdateStepEnum))))

(fn UpdateStepEnum)

(fn RunStepFirstTime
  (bind _desctextblock (Variables|Variable|GetDescTextBlock))
  (bind _steptutorialdata (Variables|Variable|GetStepTutorialData))
  (bind _titletextblock (Variables|Variable|GetTitleTextBlock))
  (bind (_title _desc) (Utilities|Struct|BreakS_TutorialStepData _steptutorialdata))
  (CallFunction|RunStep true)
  (Utilities|FlowControl|Sequence
    (:then_0
      (Utilities|IsValid _titletextblock
        (:Is%20Valid
          (if (not (Utilities|Array|IsEmpty _title))
            (Variables|/Script/UMG.TextBlock|SetText _titletextblock (Utilities|Text|ToText(String) _title))))))
    (:then_1
      (Utilities|IsValid _desctextblock
        (:Is%20Valid
          (if (not (Utilities|Array|IsEmpty _desc))
            (Variables|/Script/UMG.TextBlock|SetText _desctextblock (Utilities|Text|ToText(String) _desc))))))))

(fn RerunStep
  (CallFunction|RunStep false))

(fn RunStep
  (params (bFirstTime :type Boolean))
  (Variables|Variable|SetbFirstTime bFirstTime)
  (CallFunction|PlayDialogue))

(fn EndStep
  (CallFunction|CheckforNextStep))

(fn PlayDialogue
  (bind _steptutorialdata (Variables|Variable|GetStepTutorialData))
  (bind _dialoguecomponent (Variables|Variable|GetDialogueComponent))
  (bind (_firstdialogue _rerundialogue) (Utilities|Struct|BreakS_TutorialStepData _steptutorialdata))
  (bind _returnvalue (Utilities|Array|IsEmpty _rerundialogue))
  (Utilities|IsValid (Variables|Variable|GetDialogueComponent)
    (:Is%20Valid
      (if (or (Variables|Variable|GetbFirstTime) _returnvalue)
        (if (not (Utilities|Array|IsEmpty _firstdialogue))
          (Default|PlayDialogue _dialoguecomponent _firstdialogue))
        (elif (not _returnvalue)
          (Default|PlayDialogue _dialoguecomponent _rerundialogue))))))

(fn OnAllDialogueFinished)

(fn IsObjectiveIndexValid
  (return (>= (Variables|Variable|GetCurrentStepIndex) 0)))

(fn IsObjectiveValid
  (return true))