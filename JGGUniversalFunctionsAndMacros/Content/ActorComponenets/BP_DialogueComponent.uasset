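; Actor component that plays a sequence of dialogue lines, each with a subtitle and optional audio.
; Setup supplies the text block and audio component and binds an audio-finished event.
; Each line sets the subtitle and sound; without valid audio, a Tick countdown scaled by subtitle length advances to the next line.
; After the last line, it clears the subtitle, stops audio and signals that all dialogue has finished.
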(event EventBeginPlay)

(event EventTick
  (params (DeltaSeconds :type Float%20%28single-precision%29))
  (CallFunction|CheckGoingtoNextDialogue DeltaSeconds))

(fn Setup
  (params (SubtitleTextBlock :type Text%20Block%20Object%20Reference) (AudioComponent :type Audio%20Component%20Object%20Reference))
  (Utilities|FlowControl|Sequence
    (:then_0
      (bind _output_get (Variables|Variable|SetSubtitleTextBlock SubtitleTextBlock))
      (Utilities|IsValid _output_get
        (:Is%20Valid
          (Variables|/Script/UMG.TextBlock|SetText _output_get ""))))
    (:then_1
      (bind _output_get_2 (Variables|Variable|SetAudioComponent AudioComponent))
      (Utilities|IsValid _output_get_2
        (:Is%20Valid
          (EventDispatchers|BindEventtoOnAudioFinished _output_get_2 (EventDispatchers|CreateEvent :!event PlayDialogueLine)))))))

(fn OnAllDialogueFinished
  (CallFunction|DisableDialogue)
  (Default|CallAllDialogueFinished))

(fn PlayDialogue
  (params (Dialogue :type Array%20of%20S%20Dialogue%20Data%20Structures))
  (Variables|Variable|SetDialogue Dialogue)
  (Variables|Variable|SetbEnabled true)
  (Variables|Variable|SetDialogueIndex -1)
  (CallFunction|PlayDialogueLine))

(fn PlayDialogueLine
  (bind _dialogueindex (Variables|Variable|GetDialogueIndex))
  (bind _dialogue (Variables|Variable|GetDialogue))
  (bind _output (Utilities|Array|Get(acopy) _dialogue _dialogueindex))
  (bind (_subtitle _audio) (Utilities|Struct|BreakS_DialogueData _output))
  (Math|Integer|IncrementInt (Variables|Variable|GetDialogueIndex)
    (:%20%20
      (if (> (Utilities|Array|Length _dialogue) _dialogueindex)
        (CallFunction|ShowSubtitle _subtitle)
        (CallFunction|PlayAudio _subtitle _audio)
        (else
          (CallFunction|OnAllDialogueFinished))))))

(fn PlayAudio
  (params (Subtitle :type String) (Audio :type Sound%20Base%20Object%20Reference))
  (bind _audiocomponent (Variables|Variable|GetAudioComponent))
  (Utilities|IsValid Audio
    (:Is%20Valid
      (Utilities|IsValid _audiocomponent
        (:Is%20Valid
          (Audio|Components|Audio|SetSound _audiocomponent Audio)
          (Variables|Variable|SetbNoAudio false))
        (:Is%20Not%20Valid
          (Variables|Variable|SetbNoAudio true :!label _label)
          (Variables|Variable|SetTimeRemaining (* (Utilities|String|Len Subtitle) (Variables|Data|GetTimePerCharacterNoAudio))))))
    (:Is%20Not%20Valid
      (goto _label))))

(fn ShowSubtitle
  (params (Subtitle :type String))
  (Rendering|Components|TextRender|SetText (Variables|Variable|GetSubtitleTextBlock) (Utilities|Text|ToText(String) Subtitle)))

(fn HideSubtitle
  (Rendering|Components|TextRender|SetText (Variables|Variable|GetSubtitleTextBlock) ""))

(fn CheckGoingtoNextDialogue
  (params (Delta :type Float%20%28double-precision%29))
  (if (Math|Boolean|ANDBoolean (Variables|Variable|GetbNoAudio) (Variables|Variable|GetbEnabled) (> (Variables|Variable|GetTimeRemaining) 0.0))
    (Variables|Variable|SetTimeRemaining (- (Variables|Variable|GetTimeRemaining) Delta))
    (if (not (> (Variables|Variable|GetTimeRemaining) 0.0))
      (CallFunction|PlayDialogueLine))))

(fn DisableDialogue
  (bind _audiocomponent (Variables|Variable|GetAudioComponent))
  (Variables|Variable|SetbEnabled false)
  (CallFunction|HideSubtitle)
  (Utilities|IsValid _audiocomponent
    (:Is%20Valid
      (if (Audio|Components|Audio|IsPlaying _audiocomponent)
        (Audio|Components|Audio|Stop _audiocomponent)))))